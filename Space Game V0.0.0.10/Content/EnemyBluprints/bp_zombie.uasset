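; Zombie enemy pawn Blueprint that chases the player, hurts them on contact and dies when its health runs out.
; PawnSensing triggers an AI MoveTo toward any seen FirstPersonCharacter.
; Overlapping the ZombieHitZone subtracts a small amount from the player's Health once per overlap begin.
; Tick polls EnemyHealth and destroys the actor through a DoOnce at zero or below.
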(event `self.PawnSensing.OnSeePawn`
  (params (Pawn :type "Pawn Object Reference"))
  (bind _asfirst_person_character (cast `/Game/FirstPersonBP/Blueprints/FirstPersonCharacter` Pawn))
  (`|AIMoveTo` self (0.0 0.0 0.0) _asfirst_person_character))

(event `self.Zombie Hit Zone.OnComponentBeginOverlap`
  (params (OverlappedComponent :type "PrimitiveComponent Object Reference") (OtherActor :type "Actor Object Reference") (OtherComp :type "PrimitiveComponent Object Reference") (OtherBodyIndex :type Integer) (bFromSweep :type Boolean) (SweepResult :type "HitResult Structure (by ref)"))
  (bind _asfirst_person_character (cast `/Game/FirstPersonBP/Blueprints/FirstPersonCharacter` OtherActor))
  (set `/Game/FirstPersonBP/Blueprints/FirstPersonCharacter.Health` (- (`/Game/FirstPersonBP/Blueprints/FirstPersonCharacter.Health` _asfirst_person_character) 0.1) _asfirst_person_character))

(event `self.ReceiveTick`
  (params (DeltaSeconds :type "Float (single-precision)"))
  (bind _asbp_zombie (cast `/Game/EnemyBluprints/bp_zombie` self))
  (if (<= (`/Game/EnemyBluprints/bp_zombie.Enemy Health` _asbp_zombie) 0.0)
    (`/Engine/EditorBlueprintResources/StandardMacros.DoOnce` false
      (:`Completed`
        (`self.K2_DestroyActor` _asbp_zombie)))))

(fn `UserConstructionScript`)